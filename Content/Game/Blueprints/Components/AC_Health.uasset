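; AC_Health is an actor component that tracks health and death state for its owning actor.
; TakeDamage and GainHealth adjust health only while alive, and ResetHealth revives to MaxHealth.
; All three route through UpdateHealthAndNotify, which clamps health between zero and MaxHealth, updates IsDead, and fires OnHealthChanged and Ondeath dispatchers.
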(event `/Game/Game/Blueprints/Interfaces/BPI_Damageable.TakeDamage`
  (params (DamageAmount :type "Float (double-precision)"))
  (if (not (`self.IsDead`))
    (`self.UpdateHealthAndNotify` (- (`self.CurrentHealth`) DamageAmount))))

(event `/Game/Game/Blueprints/Interfaces/BPI_Damageable.GainHealth`
  (params (HealthAmount :type "Float (double-precision)"))
  (if (not (`self.IsDead`))
    (`self.UpdateHealthAndNotify` (+ (`self.CurrentHealth`) HealthAmount))))

(event `/Game/Game/Blueprints/Interfaces/BPI_Damageable.ResetHealth`
  (set `self.IsDead` false)
  (`self.UpdateHealthAndNotify` (`self.MaxHealth`)))

(fn `UpdateHealthAndNotify`
  (params (NewHealthValue :type "Float (double-precision)"))
  (bind _maxhealth (`self.MaxHealth`))
  (bind _output_get (set `self.CurrentHealth` (`KismetMathLibrary.FClamp` NewHealthValue 0.0 _maxhealth)))
  (`self.OnHealthChanged` _output_get _maxhealth)
  (if (<= (`self.CurrentHealth`) 0.0)
    (set `self.IsDead` true)
    (`self.Ondeath`)
    (else
      (set `self.IsDead` false))))